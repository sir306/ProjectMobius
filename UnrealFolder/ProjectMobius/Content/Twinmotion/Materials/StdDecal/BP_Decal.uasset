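; Twinmotion decal actor that passes its own rotation to its decal material.
; It creates a dynamic instance of the decal's material in both the construction script and BeginPlay, then writes the rotation to three per-axis runtime vector parameters.
; The update function can skip unchanged rotations within a small tolerance, but both live calls force it and Tick is empty, so rotation is not tracked per frame.
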(event EventBeginPlay
  ;[1 1 1] This should not exists for TM runtime
  (Decal|AssignNewDecalMaterial)
  (Decal|UpdateDynamicDecalMaterial true))

(event EventTick
  (params (DeltaSeconds :type Float%20%28single-precision%29))
  ;[1 1 1] todo: Use tick or timer events if construction script is not supported in TM runtime
)

(fn ConstructionScript
  ;[1 1 1] Warning - this recreate a material instance in the editor
  (Decal|AssignNewDecalMaterial)
  (Decal|UpdateDynamicDecalMaterial true))

(fn UpdateDynamicDecalMaterial
  (params (Force :type Boolean))
  (bind _returnvalue (Transformation|GetActorRotation))
  (Utilities|IsValid (Variables|Decal|GetDecal_MD)
    (:Is%20Valid
      (if (or Force (Utilities|Enum|NotEqual(Enum) (Variables|Decal|GetPreviousRotation) _returnvalue 0.01))
        (bind _output_get (Variables|Decal|SetPreviousRotation _returnvalue))
        (Rendering|Material|SetVectorParameterValue (Variables|Decal|GetDecal_MD) "RuntimeXAxisRot" (Math|Conversions|ToLinearColor(Vector) (.X (Math|Rotator|BreakRotIntoAxes _output_get))) :!class /Script/Engine.MaterialInstanceDynamic)
        (Rendering|Material|SetVectorParameterValue (Variables|Decal|GetDecal_MD) "RuntimeYAxisRot" (Math|Conversions|ToLinearColor(Vector) (.Y (Math|Rotator|BreakRotIntoAxes _output_get))) :!class /Script/Engine.MaterialInstanceDynamic)
        (Rendering|Material|SetVectorParameterValue (Variables|Decal|GetDecal_MD) "RuntimeZAxisRot" (Math|Conversions|ToLinearColor(Vector) (.Z (Math|Rotator|BreakRotIntoAxes _output_get))) :!class /Script/Engine.MaterialInstanceDynamic)))))

(fn AssignNewDecalMaterial
  (Utilities|IsValid (Variables|/Script/Engine.DecalComponent|GetDecalMaterial (Variables|Default|GetDecal))
    (:Is%20Valid
      ;[1 1 1] Create and assign a dynamic material from the decal material
      (bind _returnvalue (Rendering|Material|CreateDynamicMaterialInstance (Variables|/Script/Engine.DecalComponent|GetDecalMaterial (Variables|Default|GetDecal)) "None" "None" :!class /Script/Engine.KismetMaterialLibrary))
      (Variables|Decal|SetDecal_MD _returnvalue)
      (Rendering|Components|Decal|SetDecalMaterial (Variables|Default|GetDecal) (Variables|Decal|GetDecal_MD)))))