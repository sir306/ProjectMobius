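; Component that publishes the mouse cursor's position and world-space direction to materials through a Material Parameter Collection.
; Each tick it reads the viewport mouse position and deprojects it through player controller 0.
; It writes the resulting direction to CPV3_MouseDirection and the screen position, packed into red and green, to CPV3_MouseLocation.
; A debug print of the position is left unconnected.
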(event EventBeginPlay)

(event EventTick
  (params (DeltaSeconds :type Float%20%28single-precision%29))
  (bind _returnvalue (Class|WidgetLayoutLibrary|GetMousePositiononViewport))
  (Rendering|Material|SetVectorParameterValue (Variables|Default|GetMPC) (Utilities|Name|MakeLiteralName "CPV3_MouseDirection") (Math|Conversions|ToLinearColor(Vector) (.WorldDirection (Class|GameplayStatics|DeprojectScreentoWorld (Game|GetPlayerController 0) _returnvalue))) :!class /Script/Engine.KismetMaterialLibrary)
  (Rendering|Material|SetVectorParameterValue (Variables|Default|GetMPC) (Utilities|Name|MakeLiteralName "CPV3_MouseLocation") (Utilities|Struct|MakeLinearColor (.X (Math|Vector2D|BreakVector2D _returnvalue)) (.Y (Math|Vector2D|BreakVector2D _returnvalue)) 0.0 0.0) :!class /Script/Engine.KismetMaterialLibrary))