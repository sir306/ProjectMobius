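; Project Mobius player controller that creates the main UI and error popup widgets and routes keyboard shortcuts to the UI and sun control.
; On BeginPlay, if controlling a Mobius pawn, it waits a tick, adds the widgets, then caches the bottom bar and sun-rotation actor.
; Arrow keys step the bottom bar with an optional fast skip, or rotate the sun with Ctrl.
; Spacebar forwards to the UI; screenshot key and button share one capture path.
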(event Custom|Screenshot%20UI%20Button%20Clicked
  (Class|MobiusController|TakeScreenshot))

(event Input|EnhancedActionEvents|EnhancedInputActionIA_Screenshot
  (params (ActionValue :type Boolean) (ElapsedSeconds :type Float%20%28double-precision%29) (TriggeredSeconds :type Float%20%28double-precision%29) (InputAction :type Input%20Action%20Object%20Reference :default "/Game/00_UserAndInputs/InputMappings/Inputs/InputActions/IA_Screenshot.IA_Screenshot"))
  (Class|MobiusController|TakeScreenshot))

(event Input|EnhancedActionEvents|EnhancedInputActionIA_SpaceBar
  (params (ActionValue :type Boolean) (ElapsedSeconds :type Float%20%28double-precision%29) (TriggeredSeconds :type Float%20%28double-precision%29) (InputAction :type Input%20Action%20Object%20Reference :default "/Game/00_UserAndInputs/InputMappings/Inputs/InputActions/IA_SpaceBar.IA_SpaceBar"))
  (Default|CallSpacebarPressed (Variables|Default|GetWidgetWrapper)))

(event Input|EnhancedActionEvents|EnhancedInputActionIA_LeftArrow
  (params (ActionValue :type Boolean) (ElapsedSeconds :type Float%20%28double-precision%29) (TriggeredSeconds :type Float%20%28double-precision%29) (InputAction :type Input%20Action%20Object%20Reference :default "/Game/00_UserAndInputs/InputMappings/Inputs/InputActions/IA_LeftArrow.IA_LeftArrow"))
  (bind _bottom_ui_bar (Variables|Default|GetBottom%20UI%20Bar))
  (if (Input|EnhancedActionValues|GetIA_CtrlKeyModifier)
    (Class|BPIUpdateSunRotation|UpdateSunRotation(Message) (Variables|Default|GetSunDial) -1e+01)
    (elif (Utilities|PlayBarFastSkip?)
      (Class|BPIUIInterface|LeftArrow(Message) _bottom_ui_bar 5)
      (else
        (Class|BPIUIInterface|LeftArrow(Message) _bottom_ui_bar 1)))))

(event Input|EnhancedActionEvents|EnhancedInputActionIA_RightArrow
  (params (ActionValue :type Boolean) (ElapsedSeconds :type Float%20%28double-precision%29) (TriggeredSeconds :type Float%20%28double-precision%29) (InputAction :type Input%20Action%20Object%20Reference :default "/Game/00_UserAndInputs/InputMappings/Inputs/InputActions/IA_RightArrow.IA_RightArrow"))
  (bind _bottom_ui_bar (Variables|Default|GetBottom%20UI%20Bar))
  (if (Input|EnhancedActionValues|GetIA_CtrlKeyModifier)
    (Class|BPIUpdateSunRotation|UpdateSunRotation(Message) (Variables|Default|GetSunDial) 1e+01)
    (elif (Utilities|PlayBarFastSkip?)
      (Default|RightArrow _bottom_ui_bar 5)
      (else
        (Default|RightArrow _bottom_ui_bar 1)))))

(event EventBeginPlay
  (Utilities|Casting|CastToBP_MobiusPawn (Pawn|GetControlledPawn self))
  (Utilities|FlowControl|DelayUntilNextTick)
  (bind _returnvalue (Game|ConstructObjectfromClass "/Game/01_Dev/Widgets/WBP_CompleteMobiusUI.WBP_CompleteMobiusUI_C"))
  (Variables|Default|SetWidgetWrapper _returnvalue)
  (UserInterface|Viewport|AddtoViewport _returnvalue 0)
  (bind _returnvalue_2 (Game|ConstructObjectfromClass "/Game/01_Dev/Widgets/Components/Error/WBP_ErrorPopup1.WBP_ErrorPopup1_C"))
  (UserInterface|Viewport|AddtoViewport _returnvalue_2 0)
  (bind _foundwidgets (Widget|GetAllWidgetsOfClass "/Game/01_Dev/Widgets/Components/00_BottomUI/WBP_MobiusBottomBar.WBP_MobiusBottomBar_C" false))
  (bind _output_get (Variables|Default|SetBottom%20UI%20Bar (Utilities|Array|Get(acopy) _foundwidgets)))
  (EventDispatchers|BindEventtoOnClicked (Variables|/Game/01_Dev/Widgets/Components/00_BottomUI/WBP_MobiusBottomBar.WBP_MobiusBottomBar_C|GetScreenshotShortcut_Btn _output_get) (EventDispatchers|CreateEvent :!event Custom|Screenshot%20UI%20Button%20Clicked))
  (bind _outactors (Actor|GetAllActorswithInterface "/Game/01_Dev/Interfaces/BPI_UpdateSunRotation.BPI_UpdateSunRotation_C"))
  (Variables|Default|SetSunDial (Utilities|Array|Get(acopy) _outactors)))

(event EventTick
  (params (DeltaSeconds :type Float%20%28single-precision%29)))

(fn ConstructionScript)