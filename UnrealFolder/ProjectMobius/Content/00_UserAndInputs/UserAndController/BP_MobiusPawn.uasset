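; Player pawn for a free-flying camera, driven by Enhanced Input to pan, zoom and rotate, with Escape quitting the game.
; Modifier inputs switch modes and boost speed; the scene root takes movement and yaw, the spring arm pitch.
; Rotate input with right mouse held orbits a point ahead by briefly extending the spring arm, then collapsing it.
; Jump-flood render-target functions remain but are never run, noted for moving to C++ heatmap code.
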(event Input|EnhancedActionEvents|EnhancedInputActionIA_CameraMove
  (params (ActionValue :type Vector%202D%20Structure) (ElapsedSeconds :type Float%20%28double-precision%29) (TriggeredSeconds :type Float%20%28double-precision%29) (InputAction :type Input%20Action%20Object%20Reference :default "/Game/00_UserAndInputs/InputMappings/Inputs/InputActions/IA_CameraMove.IA_CameraMove"))
  (if (Input|EnhancedActionValues|GetIA_RightMouseButton)
    (CallFunction|MoveCamera 0.0 (.y ActionValue) (.x ActionValue))
    (else
      (CallFunction|MoveCamera 0.0 (.y ActionValue) 0.0)
      (CallFunction|CameraZoom (.x ActionValue)))))

(event Input|EnhancedActionEvents|EnhancedInputActionIA_CameraRotate
  (params (ActionValue :type Float%20%28double-precision%29) (ElapsedSeconds :type Float%20%28double-precision%29) (TriggeredSeconds :type Float%20%28double-precision%29) (InputAction :type Input%20Action%20Object%20Reference :default "/Game/00_UserAndInputs/InputMappings/Inputs/InputActions/IA_CameraRotate.IA_CameraRotate"))
  (if (Input|EnhancedActionValues|GetIA_RightMouseButton)
    (CallFunction|SpringArmRotation ActionValue)
    (else
      (CallFunction|ImpRotateCamera 0.0 0.0 ActionValue))))

(event Input|EnhancedActionEvents|EnhancedInputActionIA_CameraZoom
  (params (ActionValue :type Vector%202D%20Structure) (ElapsedSeconds :type Float%20%28double-precision%29) (TriggeredSeconds :type Float%20%28double-precision%29) (InputAction :type Input%20Action%20Object%20Reference :default "/Game/00_UserAndInputs/InputMappings/Inputs/InputActions/IA_CameraZoom.IA_CameraZoom"))
  (if (not (Variables|Default|GetMouse%20on%20UI?))
    (CallFunction|CameraZoom (.x ActionValue))))

(event Input|EnhancedActionEvents|EnhancedInputActionIA_MouseMovement
  (params (ActionValue :type Vector%202D%20Structure) (ElapsedSeconds :type Float%20%28double-precision%29) (TriggeredSeconds :type Float%20%28double-precision%29) (InputAction :type Input%20Action%20Object%20Reference :default "/Game/00_UserAndInputs/InputMappings/Inputs/InputActions/IA_MouseMovement.IA_MouseMovement"))
  (bind (_x _y) (Math|Vector2D|BreakVector2D ActionValue))
  ;[0.2 0.1763 0.02039 1 12] Middle and Rmb can both be held so need to do rotate and move, its unlikely and will cause weird movements but to avoid favouring one movement over the other this is the best way to do so
  (Utilities|FlowControl|Sequence
    (:then_0
      (if (Input|EnhancedActionValues|GetIA_RightMouseButton)
        (CallFunction|MouseRmbRotateView ActionValue)))
    (:then_1
      (if (Input|EnhancedActionValues|GetIA_MiddleMouseButton)
        (CallFunction|MoveCamera 0.0 _x _y)))))

(event Input|EnhancedActionEvents|EnhancedInputActionIA_R_Key
  (params (ActionValue :type Boolean) (ElapsedSeconds :type Float%20%28double-precision%29) (TriggeredSeconds :type Float%20%28double-precision%29) (InputAction :type Input%20Action%20Object%20Reference :default "/Game/00_UserAndInputs/InputMappings/Inputs/InputActions/IA_R_Key.IA_R_Key"))
  (if (Input|EnhancedActionValues|GetIA_CtrlKeyModifier)
    (Transformation|SetWorldRotation (Variables|Default|GetDefaultSceneRoot) "0, 0, 0" false false)
    (Transformation|SetRelativeRotation (Variables|Default|GetSpringArm) "0, 0, 0" false false)))

(event EventBeginPlay
  (bind _returnvalue (Game|GetPlayerController 0))
  (Input|EnableInput _returnvalue)
  (Input|AddMappingContext (PlayerController|LocalPlayerSubsystems|GetEnhancedInputLocalPlayerSubsystem _returnvalue) "/Game/00_UserAndInputs/InputMappings/Inputs/InputMappings/IMC_UserControl.IMC_UserControl" 0 "(bIgnoreAllPressedKeysUntilRelease=True,bForceImmediately=False,bNotifyUserSettings=False)"))

(event Collision|EventActorBeginOverlap
  (params (OtherActor :type Actor%20Object%20Reference)))

(event EventTick
  (params (DeltaSeconds :type Float%20%28single-precision%29)))

(event EventMouseonUIElement?
  (params (MouseOnUI? :type Boolean))
  (Variables|Default|SetMouse%20on%20UI? MouseOnUI?))

(event Input|KeyboardEvents|Escape
  (params (Key :type Key%20Structure))
  (:Pressed
    (Game|QuitGame 0 "Quit" false)))

(event Input|KeyboardEvents|NumPadOne
  (params (Key :type Key%20Structure))
  ;[0.01096 0.01161 0.0137] Move to heatmap c++ code
)

(event Input|KeyboardEvents|NumPadTwo
  (params (Key :type Key%20Structure))
  ;[0.01096 0.01161 0.0137] Move to heatmap c++ code
)

(event Input|KeyboardEvents|NumPadThree
  (params (Key :type Key%20Structure))
  ;[0.01096 0.01161 0.0137] Move to heatmap c++ code
)

(fn ConstructionScript)

(fn InitRT
  (Rendering|ClearRenderTarget2D "/Game/01_Dev/NickMaster/Heatmaps/Materials/JFA_VoronoiTest/RT_JFA_test.RT_JFA_test")
  (bind (_canvas _size _context) (Rendering|BeginDrawCanvastoRenderTarget "/Game/01_Dev/NickMaster/Heatmaps/Materials/JFA_VoronoiTest/RT_JFA_test.RT_JFA_test"))
  (Canvas|DrawMaterial :self _canvas :RenderMaterial "/Game/01_Dev/NickMaster/Heatmaps/Materials/JFA_VoronoiTest/M_JFA_Init.M_JFA_Init" :ScreenSize _size :CoordinateSize "(X=1.000000,Y=1.000000)" :PivotPoint "(X=0.500000,Y=0.500000)")
  (Rendering|EndDrawCanvastoRenderTarget _context))

(fn JFAUpdate
  (bind _dmi_jfa_test (Variables|Default|GetDMI_JFA_test))
  (for _index (range 1 (Math|Float|Truncate (Math|Float|Log (Variables|Default|Gettexturesize) 2.0)))
    (Rendering|Material|SetScalarParameterValue _dmi_jfa_test "Step" (/ 1.0 (Math|Float|Power 2.0 (Math|Conversions|ToFloat(Integer) _index))) :!class /Script/Engine.MaterialInstanceDynamic)
    (bind (_canvas _size _context) (Rendering|BeginDrawCanvastoRenderTarget "/Game/01_Dev/NickMaster/Heatmaps/Materials/JFA_VoronoiTest/RT_JFA_test.RT_JFA_test"))
    (Canvas|DrawMaterial :self _canvas :RenderMaterial _dmi_jfa_test :ScreenSize _size :CoordinateSize "(X=1.000000,Y=1.000000)" :PivotPoint "(X=0.500000,Y=0.500000)")
    (Rendering|EndDrawCanvastoRenderTarget _context)))

(fn CameraZoom
  (params (AxisVal :type Float%20%28double-precision%29))
  (bind _camera (Variables|Default|GetCamera))
  (bind _camerazoomspeedoffset (Variables|Default|GetCameraZoomSpeedOffset))
  (bind _defaultsceneroot (Variables|Default|GetDefaultSceneRoot))
  (bind _returnvalue (Math|Vector|GetForwardVector _camera))
  ;[0.01096 0.01161 0.0137] Don't want to zoom when holding mouse button
  (if (not (Input|EnhancedActionValues|GetIA_MiddleMouseButton))
    (if (Input|EnhancedActionValues|GetIA_IncreaseMovementSpeed)
      (Transformation|AddWorldOffset _defaultsceneroot (* _returnvalue (* AxisVal _camerazoomspeedoffset (Variables|Default|GetIncreasedMovementSpeedMultiplier))) false false)
      (else
        (Transformation|AddWorldOffset _defaultsceneroot (* _returnvalue (* AxisVal _camerazoomspeedoffset)) false false)))))

(fn MouseRmbRotateView
  (params (MouseAxisValues :type Vector%202D%20Structure))
  (bind (_x _y) (Math|Vector2D|BreakVector2D MouseAxisValues))
  (CallFunction|ImpRotateCamera 0.0 _y _x))

(fn MoveCamera
  (params (X :type Float%20%28double-precision%29) (Y :type Float%20%28double-precision%29) (Z :type Float%20%28double-precision%29))
  (CallFunction|ImpCameraMove X Y Z)
  (return))

(fn ImpCameraMove
  (params (X :type Float%20%28double-precision%29) (Y :type Float%20%28double-precision%29) (Z :type Float%20%28double-precision%29))
  (bind _camera (Variables|Default|GetCamera))
  (bind _cameramovementspeedoffset (Variables|Default|GetCameraMovementSpeedOffset))
  (bind _increasedmovementspeedmultiplier (Variables|Default|GetIncreasedMovementSpeedMultiplier))
  (bind _defaultsceneroot (Variables|Default|GetDefaultSceneRoot))
  (bind _returnvalue (Transformation|GetWorldRotation _defaultsceneroot))
  (bind _returnvalue_2 (Math|Vector|GetForwardVector _camera))
  (bind _returnvalue_3 (Math|Conversions|RotationFromXVector _returnvalue_2))
  ;[0.01096 0.01161 0.0137] Mouse button not held so we want to move and not zoom
  (if (Input|EnhancedActionValues|GetIA_IncreaseMovementSpeed)
    (Transformation|AddWorldOffset _defaultsceneroot (Math|Vector|RotateVector (Math|Vector|MakeVector (* X _cameramovementspeedoffset _increasedmovementspeedmultiplier) (* Y _cameramovementspeedoffset _increasedmovementspeedmultiplier) (* Z _cameramovementspeedoffset _increasedmovementspeedmultiplier)) (Math|Rotator|MakeRotator (.roll _returnvalue_3) (.pitch _returnvalue_3) (.yaw _returnvalue))) false false)
    (else
      (Transformation|AddWorldOffset _defaultsceneroot (Math|Vector|RotateVector (Math|Vector|MakeVector (* X _cameramovementspeedoffset) (* Y _cameramovementspeedoffset) (* Z _cameramovementspeedoffset)) (Math|Rotator|MakeRotator (.roll _returnvalue_3) (.pitch _returnvalue_3) (.yaw _returnvalue))) false false)))
  (return))

(fn ImpRotateCamera
  (params (Roll :type Float%20%28double-precision%29) (Pitch :type Float%20%28double-precision%29) (Yaw :type Float%20%28double-precision%29))
  (bind _springarm (Variables|Default|GetSpringArm))
  (bind _defaultsceneroot (Variables|Default|GetDefaultSceneRoot))
  (if (Input|EnhancedActionValues|GetIA_IncreaseMovementSpeed)
    (Transformation|AddWorldRotation _defaultsceneroot (Math|Rotator|MakeRotator 0.0 0.0 (* Yaw (Variables|Default|GetCameraRotateSpeedOffset) (Variables|Default|GetIncreasedMovementSpeedMultiplier))) false false)
    (Transformation|AddRelativeRotation _springarm (Math|Rotator|MakeRotator (* Roll (Variables|Default|GetCameraRotateSpeedOffset) (Variables|Default|GetIncreasedMovementSpeedMultiplier)) (Math|Float|Clamp(Float) (* Pitch (Variables|Default|GetCameraRotateSpeedOffset) (Variables|Default|GetIncreasedMovementSpeedMultiplier)) -9e+01 9e+01) 0.0) false false)
    (else
      (Transformation|AddWorldRotation _defaultsceneroot (Math|Rotator|MakeRotator 0.0 0.0 (* Yaw (Variables|Default|GetCameraRotateSpeedOffset))) false false)
      (Transformation|AddRelativeRotation _springarm (Math|Rotator|MakeRotator (* Roll (Variables|Default|GetCameraRotateSpeedOffset)) (Math|Float|Clamp(Float) (* Pitch (Variables|Default|GetCameraRotateSpeedOffset)) -9e+01 9e+01) 0.0) false false)))
  (return))

(fn SpringArmRotation
  (params (Yaw :type Float%20%28double-precision%29))
  (bind _springarm (Variables|Default|GetSpringArm))
  (CallFunction|OffsetSpringArmforRotation)
  (if (Input|EnhancedActionValues|GetIA_IncreaseMovementSpeed)
    (Transformation|AddRelativeRotation _springarm (Math|Rotator|MakeRotator 0.0 0.0 (* Yaw (Variables|Default|GetCameraRotateSpeedOffset) (Variables|Default|GetIncreasedMovementSpeedMultiplier))) false false)
    (else
      (Transformation|AddRelativeRotation _springarm (Math|Rotator|MakeRotator 0.0 0.0 (* Yaw (Variables|Default|GetCameraRotateSpeedOffset))) false false)))
  (CallFunction|ReturnSpringArmOffsettoDefault)
  (return))

(fn OffsetSpringArmforRotation
  (Transformation|AddWorldOffset (Variables|Default|GetDefaultSceneRoot) (* (Math|Vector|GetForwardVector (Variables|Default|GetCamera)) (Variables|Default|GetSpringArmExtension)) false false)
  (Variables|/Script/Engine.SpringArmComponent|SetTargetArmLength (Variables|Default|GetSpringArm) (Variables|Default|GetSpringArmExtension))
  (return))

(fn ReturnSpringArmOffsettoDefault
  (bind _camera (Variables|Default|GetCamera))
  (bind _returnvalue (Transformation|GetWorldRotation _camera))
  (Transformation|SetWorldTransform (Variables|Default|GetDefaultSceneRoot) (Math|Transform|MakeTransform (- (Transformation|GetWorldLocation (Variables|Default|GetDefaultSceneRoot)) (* (Math|Vector|GetForwardVector (Variables|Default|GetCamera)) (Variables|Default|GetSpringArmExtension))) (Math|Rotator|MakeRotator 0.0 0.0 (.yaw _returnvalue)) "1.000000,1.000000,1.000000") false false)
  (Transformation|SetRelativeRotation (Variables|Default|GetSpringArm) (Math|Rotator|MakeRotator (.roll _returnvalue) (.pitch _returnvalue) 0.0) false false)
  (Variables|/Script/Engine.SpringArmComponent|SetTargetArmLength (Variables|Default|GetSpringArm) 0.0))