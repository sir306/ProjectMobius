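; Test actor that feeds CPU-generated agent positions into a Niagara system, apparently for pedestrian movement conversion to Niagara.
; The Construction Script scatters random points on a flat square and passes their count and locations to Niagara user variables.
; Tick shifts every point along the positive XY diagonal, scaled by delta time, then re-pushes the whole AgentLocations array.
; The ParticleData event is an empty stub.
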(event EventBeginPlay)

(event Collision|EventActorBeginOverlap
  (params (OtherActor :type Actor%20Object%20Reference)))

(event EventTick
  (params (DeltaSeconds :type Float%20%28single-precision%29))
  (bind _returnvalue (/ 1.2e+02 DeltaSeconds))
  (bind _returnvalue_2 (/ 5e+02 _returnvalue))
  (for (_array_element _array_index) (Variables|Default|GetTest%20Location%20Array%20Data)
    (Utilities|Array|SetArrayElem (Variables|Default|GetTest%20Location%20Array%20Data) _array_index (+ _array_element (Math|Vector|MakeVector _returnvalue_2 _returnvalue_2 0.0))))
  (Class|NiagaraDataInterfaceArrayFunctionLibrary|SetNiagaraArrayVector (Variables|Default|GetNiagara) "AgentLocations" (Variables|Default|GetTest%20Location%20Array%20Data)))

(event EventParticleData
  (params (Data :type Array%20of%20Basic%20Particle%20Data%20Structures) (NiagaraSystem :type Niagara%20System%20Object%20Reference) (SimulationPositionOffset :type Vector%20%28by%20ref%29 :default "0, 0, 0")))

(fn ConstructionScript
  (bind _niagara (Variables|Default|GetNiagara))
  (bind _test_location_array_data (Variables|Default|GetTest%20Location%20Array%20Data))
  (Utilities|Array|Clear (Variables|Default|GetTest%20Location%20Array%20Data))
  (for _index (range 0 50)
    (Utilities|Array|Add (Variables|Default|GetTest%20Location%20Array%20Data) (Math|Vector|MakeVector (Math|Random|RandomFloatinRange -5e+02 5e+02) (Math|Random|RandomFloatinRange -5e+02 5e+02) 0.0)))
  (Class|NiagaraComponent|SetVariableInt _niagara "NumberOfAgents" (Utilities|Array|Length _test_location_array_data))
  (Class|NiagaraDataInterfaceArrayFunctionLibrary|SetNiagaraArrayVector _niagara "AgentLocations" _test_location_array_data))