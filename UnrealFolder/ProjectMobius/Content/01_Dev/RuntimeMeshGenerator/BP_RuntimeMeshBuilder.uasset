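; Runtime mesh builder actor for Project Mobius that loads simulation geometry from file into a procedural mesh component.
; BuildMeshFromFile clears existing sections, garbage collects, then reads mesh data with a 90-degree rotation; ClearMesh only clears and collects.
; OnMeshBuilt_Event cycles Datasmith material styles to precompile shaders and reduce packaged-build stutter, though its binding here is disconnected.
; Other disconnected chains hold test paths, debug views and mesh experiments.
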(event Custom|BuildMeshFromFile
  (Utilities|ClearAllMeshSectionsandCollectGarbage)
  (Class|RuntimeMeshBuilder|GetMeshDatafromFile "0.000000,0.000000,90.000000"))

(event Custom|ClearMesh
  (Utilities|ClearAllMeshSectionsandCollectGarbage))

(event Custom|OnMeshBuilt_Event
  (params (BoundOrigins :type Vector) (BoundExtents :type Vector))
  ;[0.01096 0.01161 0.0137] This trick should make the shaders compile when first ran and should eliviate the stuttering problem in the package, it will cause it to take longer at startup but should aid the execution of it
  (Class|RuntimeMeshBuilder|SetDatasmithMeshtoSolidMaterials)
  (Class|RuntimeMeshBuilder|SetDatasmithMeshtoTranslucentMaterials)
  (Class|RuntimeMeshBuilder|SetDatasmithtoUseModifiedColour true "(R=1.000000,G=1.000000,B=1.000000,A=1.000000)")
  (Class|RuntimeMeshBuilder|SetDatasmithtoUseModifiedColour false "(R=1.000000,G=1.000000,B=1.000000,A=1.000000)")
  (Class|RuntimeMeshBuilder|SetDatasmithMeshtoUseNonModifiedMaterials false)
  (Class|RuntimeMeshBuilder|SetDatasmithtoOriginalMatStyle))

(event EventBeginPlay)

(event Collision|EventActorBeginOverlap
  (params (OtherActor :type Actor%20Object%20Reference)))

(event EventTick
  (params (DeltaSeconds :type Float%20%28single-precision%29)))

(fn ConstructionScript)