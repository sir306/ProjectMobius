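; Test actor that procedurally builds a flat grid mesh on its RuntimeHeatmapMeshComponent in the Construction Script, with no runtime logic.
; It derives cell size from DesiredSize, XCount and YCount, then fills row-major vertices, normalized UVs and two triangles per cell.
; An experimental trim pass drops individual indices, rather than whole triangles, whose values fall in a range based on index count before creating the section.
; A hardcoded test quad is created and immediately cleared beforehand.
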(event EventBeginPlay)

(event Collision|EventActorBeginOverlap
  (params (OtherActor :type Actor%20Object%20Reference)))

(event EventTick
  (params (DeltaSeconds :type Float%20%28single-precision%29)))

(fn ConstructionScript
  (bind _x_count (LocalVariables|GetX%20count))
  (bind _triangleindexs (Variables|Default|GetTriangleIndexs))
  (bind _runtimeheatmapmeshcomponent (Variables|Default|GetRuntimeHeatmapMeshComponent))
  (bind _desired_size (LocalVariables|GetDesired%20Size))
  (bind _triangleindexs_2 (Variables|Default|GetTriangleIndexs))
  (bind _triangleindexs_3 (Variables|Default|GetTriangleIndexs))
  (bind _returnvalue (Utilities|Array|Length _triangleindexs_2))
  (Class|ProceduralMeshComponent|ClearMeshSection _runtimeheatmapmeshcomponent)
  (Class|ProceduralMeshComponent|CreateMeshSectionLinearColor _runtimeheatmapmeshcomponent 0 (Utilities|Array|MakeArray "0, 0, 0" "1000.000000,0.000000,0.000000" "1000.000000,1000.000000,0.000000" "0.000000,1000.000000,0.000000") (Utilities|Array|MakeArray 0 2 1 0 3 2) 0 (Utilities|Array|MakeArray "" "(X=1.000000,Y=0.000000)" "(X=1.000000,Y=1.000000)" "(X=0.000000,Y=1.000000)") 0 0 0 0 0 false false)
  (Class|ProceduralMeshComponent|ClearMeshSection _runtimeheatmapmeshcomponent)
  (bind _output_get (LocalVariables|SetCellSize (Math|Vector2D|MakeVector2D (/ (.x _desired_size) (LocalVariables|GetX%20count)) (/ (.y _desired_size) (LocalVariables|GetY%20count)))))
  (bind _output_get_2 (LocalVariables|SetCellOffset (Math|Vector2D|MakeVector2D (/ (.x (LocalVariables|GetCellSize)) (- (LocalVariables|GetX%20count) 1)) (/ (.y (LocalVariables|GetCellSize)) (- (LocalVariables|GetY%20count) 1)))))
  (LocalVariables|SetCellSize (+ _output_get_2 _output_get))
  (Utilities|Array|Clear (Variables|Default|GetUVs))
  (Utilities|Array|Clear (Variables|Default|GetTriangleIndexs))
  (Utilities|Array|Clear (Variables|Default|GetVertices))
  (for _index (range 0 (- (LocalVariables|GetY%20count) 1))
    (for _index_2 (range 0 (- (LocalVariables|GetX%20count) 1))
      (Utilities|Array|Add (Variables|Default|GetVertices) (Math|Vector|MakeVector (Math|Conversions|ToFloat(Integer) (* _index_2 (.x (LocalVariables|GetCellSize)))) (Math|Conversions|ToFloat(Integer) (* _index (.y (LocalVariables|GetCellSize)))) 0.0))
      (Utilities|Array|Add (Variables|Default|GetUVs) (Math|Vector2D|MakeVector2D (/ (Math|Conversions|ToFloat(Integer) (* _index_2 (.x (LocalVariables|GetCellSize)))) (* (- (LocalVariables|GetX%20count) 1) (.x (LocalVariables|GetCellSize)))) (/ (Math|Conversions|ToFloat(Integer) (* _index (.y (LocalVariables|GetCellSize)))) (* (- (LocalVariables|GetY%20count) 1) (.y (LocalVariables|GetCellSize))))))))
  (for _index_3 (range 0 (- (LocalVariables|GetY%20count) 2))
    (for _index_4 (range 0 (- (LocalVariables|GetX%20count) 2))
      (Utilities|Array|Add _triangleindexs (+ _index_4 (* _index_3 _x_count)))
      (Utilities|Array|Add _triangleindexs (+ (+ _index_4 (* _index_3 _x_count)) _x_count))
      (Utilities|Array|Add _triangleindexs (+ (+ _index_4 (* _index_3 _x_count)) 1))
      (Utilities|Array|Add _triangleindexs_3 (+ (+ _index_4 (* _index_3 _x_count)) _x_count))
      (Utilities|Array|Add _triangleindexs_3 (+ (+ (+ _index_4 (* _index_3 _x_count)) _x_count) 1))
      (Utilities|Array|Add _triangleindexs_3 (+ (+ _index_4 (* _index_3 _x_count)) 1))))
  (Utilities|Array|Clear (Variables|Default|GetTrim))
  (for _index_5 (range 0 _returnvalue)
    (if (not (Math|Integer|InRange(Integer) (Utilities|Array|Get(acopy) _triangleindexs_2 _index_5) (/ _returnvalue 12) (/ _returnvalue 6)))
      (Utilities|Array|Add (Variables|Default|GetTrim) (Utilities|Array|Get(acopy) _triangleindexs_2 _index_5))))
  (Class|ProceduralMeshComponent|CreateMeshSectionLinearColor (Variables|Default|GetRuntimeHeatmapMeshComponent) 0 (Variables|Default|GetVertices) (Variables|Default|GetTrim) 0 (Variables|Default|GetUVs) 0 0 0 0 0 false false))