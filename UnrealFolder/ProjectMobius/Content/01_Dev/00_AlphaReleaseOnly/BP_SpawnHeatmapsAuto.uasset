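; Alpha-only helper actor that sizes and places heatmaps automatically from the runtime-built mesh.
; On BeginPlay it waits a tick, finds the BP_RuntimeMeshBuilder and binds to its OnMeshBuilt event.
; When the mesh is built, it passes the origin and box extent to the Heatmap Subsystem as spawn location and size.
; Older logic that spawned per-floor HeatmapPixelTextureVisualizer actors remains disconnected.
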(event Custom|Mesh%20has%20been%20built
  (params (Origin :type Vector) (Box%20Extent :type Vector))
  (Class|HeatmapSubsystem|UpdateSpawnLocationandHeatmapSize (Subsystems|GetHeatmapSubsystem) Origin Box%20Extent)
  (Utilities|FlowControl|Delay 3.0))

(event EventBeginPlay
  (Utilities|FlowControl|Delay 0.0)
  (bind _returnvalue (Actor|GetActorOfClass "/Game/01_Dev/RuntimeMeshGenerator/BP_RuntimeMeshBuilder.BP_RuntimeMeshBuilder_C"))
  (if (Utilities|IsValid _returnvalue)
    (bind _output_get (Variables|Default|SetAs%20BP%20Runtime%20Mesh%20Builder _returnvalue))
    (EventDispatchers|BindEventtoOnMeshBuilt _output_get (EventDispatchers|CreateEvent :!event Custom|Mesh%20has%20been%20built))))

(event Collision|EventActorBeginOverlap
  (params (OtherActor :type Actor%20Object%20Reference)))

(event EventTick
  (params (DeltaSeconds :type Float%20%28single-precision%29)))

(fn ConstructionScript)