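; Sequencer scripting helpers in the mocap tools for locating FK Control Rig data in a sequence.
; GetFKTracks searches the first binding's tracks for a row named "FKControlRig" and returns that track's sections with a success flag, exiting before later bindings are checked.
; A separate helper reports whether a channel name contains any of the given substrings.
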(fn GetFKTracks
  (params (Sequence :type Movie%20Scene%20Sequence%20Object%20Reference))
  (bind _returnvalue (Class|MovieSceneSequenceExtensions|GetBindings Sequence))
  (for _array_element _returnvalue
    (bind _returnvalue_2 (Class|MovieSceneBindingExtensions|GetTracks _array_element))
    (bind (_array_element_2 _array_index) (Utilities|Array|ForEachLoopwithBreak _returnvalue_2 :!label _label)
      (:LoopBody
        (bind _returnvalue_3 (Class|MovieSceneTrackExtensions|GetTrackRowDisplayName _array_element_2 _array_index))
        (bind _output_get (LocalVariables|SetFound (Utilities|Enum|Equal(Enum) _returnvalue_3 (Utilities|Text|MakeLiteralText "FKControlRig"))))
        (if _output_get
          (bind _returnvalue_4 (Class|MovieSceneTrackExtensions|GetSections _array_element_2))
          (LocalVariables|SetTracks _returnvalue_4)
          (goto _label Break)))
      (:Completed
        (return (LocalVariables|GetTracks) (LocalVariables|GetFound)))))
  (Development|PrintString 0 "Done"))

(fn FKChannelMatchesContainsString
  (params (SearchIn :type String) (Substrings :type Array%20of%20Strings))
  (bind _array_element (Utilities|Array|ForEachLoopwithBreak Substrings :!label _label)
    (:LoopBody
      (bind _output_get (LocalVariables|SetFound (Utilities|String|Contains SearchIn _array_element)))
      (if _output_get
        (goto _label Break)))
    (:Completed
      (return (LocalVariables|GetFound)))))