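; Prototype actor that draws a 3D line graph with spline meshes inside a configurable box, along X or Y.
; The construction script sizes background and axes, spaces random-height points by count or distance, builds mesh segments and applies dynamic grid materials.
; Construction and BeginPlay feed test locations into SplineGraphLocationBucket, print counts and set the last point's height from bucket 0's count.
; Quad-tree density test code is left disconnected.
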(event EventBeginPlay
  (bind _splinegraphlocationbucket (Variables|Default|GetSplineGraphLocationBucket))
  (bind _defaultsceneroot (Variables|Default|GetDefaultSceneRoot))
  (bind _splineplothelper (Variables|Default|GetSplinePlotHelper))
  (bind _returnvalue (Transformation|GetWorldLocation _defaultsceneroot))
  (bind _returnvalue_2 (Spline|GetNumberOfSplinePoints _splineplothelper))
  (bind _returnvalue_3 (- _returnvalue_2 1))
  (bind _returnvalue_4 (Spline|GetSplinePointAt _splineplothelper _returnvalue_3 "Local"))
  (Class|SplineGraphLocationBucket|CreateSplineGraphLocationBuckets _splinegraphlocationbucket _returnvalue (* (Variables|/Script/Engine.BoxComponent|GetBoxExtent (Variables|Default|GetBox)) 2) 8 (Variables|Default|GetXGraph))
  (for _index (range 0 50)
    (Utilities|FlowControl|Delay 0.0)
    (Class|SplineGraphLocationBucket|AddEntitytoBucket _splinegraphlocationbucket (+ _returnvalue (Math|Vector|MakeVector (* _index 10) 0.0 0.0)))
    (bind _returnvalue_5 (Class|SplineGraphLocationBucket|GetTotalEntitiesinSegmentBucket _splinegraphlocationbucket))
    (Development|PrintString (Utilities|String|Append "Number of entities: " (Utilities|String|ToString(Integer) _returnvalue_5)))
    (CallFunction|UpdateSplinePoint _returnvalue_3 (Math|Vector|MakeVector (.x (.position _returnvalue_4)) (.y (.position _returnvalue_4)) (* (+ (.Z (Math|Vector|BreakVector _returnvalue)) 75.0) _returnvalue_5)) (.arrivetangent _returnvalue_4))
    (for _index_2 (range 0 _returnvalue_3)
      (CallFunction|UpdateSplineMeshComponent _index_2))))

(event Collision|EventActorBeginOverlap
  (params (OtherActor :type Actor%20Object%20Reference)))

(event EventTick
  (params (DeltaSeconds :type Float%20%28single-precision%29)))

(fn ConstructionScript
  (bind _splinegraphlocationbucket (Variables|Default|GetSplineGraphLocationBucket))
  (bind _defaultsceneroot (Variables|Default|GetDefaultSceneRoot))
  (bind _userdataoffsetdistance (Variables|Default|GetUserDataOffsetDistance))
  (bind _userdataoffsetdistance_2 (Variables|Default|GetUserDataOffsetDistance))
  (bind _splinegraphlocationbucket_2 (Variables|Default|GetSplineGraphLocationBucket))
  (bind _graphsplinemesh (Variables|Default|GetGraphSplineMesh))
  (bind _graphbackground (Variables|Default|GetGraphBackGround))
  (bind _splineplothelper (Variables|Default|GetSplinePlotHelper))
  (bind _xaxis (Variables|Default|GetXAxis))
  (bind _yaxis (Variables|Default|GetYAxis))
  (bind _xgraphaxisoffset (Variables|Default|GetXGraphAxisOffset))
  (bind _box (Variables|Default|GetBox))
  (bind _box_2 (Variables|Default|GetBox))
  (bind _returnvalue (Transformation|GetWorldLocation _defaultsceneroot))
  (bind _returnvalue_2 (Spline|GetNumberOfSplinePoints _splineplothelper))
  (bind _boxextent (Variables|/Script/Engine.BoxComponent|GetBoxExtent _box_2))
  (bind (_x _y _z) (Math|Vector|BreakVector _boxextent))
  (bind _returnvalue_3 (- _returnvalue_2 1))
  (bind _returnvalue_4 (Spline|GetSplinePointAt _splineplothelper _returnvalue_3 "Local"))
  (bind _returnvalue_5 (/ _z 5e+01))
  (bind _returnvalue_6 (/ _y 5e+01))
  (for _array_element _graphsplinemesh
    (Components|DestroyComponent _array_element))
  (Utilities|Array|Clear _graphsplinemesh)
  (Components|Box|SetBoxExtent _box (Variables|Default|GetDetectionBoxSize) true)
  (Transformation|SetRelativeLocation _box "0, 0, 0" false true)
  (Transformation|AddLocalOffset _box _boxextent false true)
  (Variables|Default|SetBoxSize (* _boxextent 2))
  (Variables|Default|SetStartPos (- (Variables|/Script/Engine.SceneComponent|GetRelativeLocation _box_2) _boxextent))
  (Utilities|GraphType-XTop
    (:X-Axis
      (Transformation|SetRelativeTransform _graphbackground (Math|Transform|MakeTransform (+ (Variables|Default|GetStartPos) (Math|Vector|MakeVector _x 0.0 _z)) "0.000000,0.000000,-90.000000" (Math|Vector|MakeVector _returnvalue_6 _returnvalue_5 _returnvalue_5)) false false)
      (Transformation|SetRelativeTransform _xaxis (Math|Transform|MakeTransform (- (+ (Variables|Default|GetStartPos) (Math|Vector|MakeVector _x 0.0 0.0)) (Math|Vector|MakeVector 0.0 0.0 _xgraphaxisoffset)) "0.000000,0.000000,-90.000000" (Math|Vector|MakeVector _returnvalue_6 0.1 1.0)) false false)
      (Transformation|SetRelativeTransform _yaxis (Math|Transform|MakeTransform (+ (+ (Variables|Default|GetStartPos) (Math|Vector|MakeVector 0.0 0.0 _z)) (Math|Vector|MakeVector (+ (* _x 2) (Variables|Default|GetXGraphAxisOffset)) 0.0 0.0)) "-90.000000,-90.000000,0.000000" (Math|Vector|MakeVector _returnvalue_5 0.1 1.0)) false false))
    (:Y-Axis
      (Transformation|SetRelativeTransform _graphbackground (Math|Transform|MakeTransform (+ (Variables|Default|GetStartPos) (Math|Vector|MakeVector 0.0 _y _z)) "90.000000,0.000000,0.000000" (Math|Vector|MakeVector _returnvalue_5 _returnvalue_6 _returnvalue_5)) false false)
      (Transformation|SetRelativeTransform _xaxis (Math|Transform|MakeTransform (- (+ (Variables|Default|GetStartPos) (Math|Vector|MakeVector 0.0 _y 0.0)) (Math|Vector|MakeVector 0.0 0.0 _xgraphaxisoffset)) "90.000000,0.000000,0.000000" (Math|Vector|MakeVector 0.1 _returnvalue_6 1.0)) false false)
      (Transformation|SetRelativeTransform _yaxis (Math|Transform|MakeTransform (- (+ (Variables|Default|GetStartPos) (Math|Vector|MakeVector 0.0 0.0 _z)) (Math|Vector|MakeVector 0.0 (Variables|Default|GetXGraphAxisOffset) 0.0)) "0.000000,-90.000000,-90.000000" (Math|Vector|MakeVector 0.1 _returnvalue_5 1.0)) false false)))
  (Variables|Default|SetNumberOfDataPoints (Variables|Default|GetUserNumberOfDataPoints))
  (if (not (Variables|Default|GetUseNumOfPoints?))
    (Utilities|GraphType-XTop
      (:X-Axis
        (Variables|Default|SetDataOffsetDistance (+ _userdataoffsetdistance (/ (.Remainder (Math|Float|Division(WholeandRemainder) (.x (Variables|Default|GetBoxSize)) _userdataoffsetdistance_2)) (.ReturnValue (Math|Float|Division(WholeandRemainder) (.x (Variables|Default|GetBoxSize)) _userdataoffsetdistance_2))))))
      (:Y-Axis
        (Variables|Default|SetDataOffsetDistance (+ _userdataoffsetdistance (/ (.Remainder (Math|Float|Division(WholeandRemainder) (.y (Variables|Default|GetBoxSize)) _userdataoffsetdistance_2)) (.ReturnValue (Math|Float|Division(WholeandRemainder) (.y (Variables|Default|GetBoxSize)) _userdataoffsetdistance_2))))))))
  (if (> (Variables|Default|GetDataOffsetDistance) 0.0)
    _
    (else
      (Variables|Default|SetDataOffsetDistance 1.0)))
  (if (> (Variables|Default|GetNumberOfDataPoints) 2)
    _
    (else
      (Variables|Default|SetNumberOfDataPoints 2)))
  (if (Variables|Default|GetUseNumOfPoints?)
    (Utilities|GraphType-XTop
      (:X-Axis
        (Variables|Default|SetDataOffsetDistance (/ (.x (Variables|Default|GetBoxSize)) (- (Variables|Default|GetNumberOfDataPoints) 1))))
      (:Y-Axis
        (Variables|Default|SetDataOffsetDistance (/ (.y (Variables|Default|GetBoxSize)) (- (Variables|Default|GetNumberOfDataPoints) 1)))))
    (else
      (Utilities|GraphType-XTop
        (:X-Axis
          (Variables|Default|SetNumberOfDataPoints (+ (Math|Float|Truncate (/ (.x (Variables|Default|GetBoxSize)) (Variables|Default|GetDataOffsetDistance))) 1)))
        (:Y-Axis
          (Variables|Default|SetNumberOfDataPoints (+ (Math|Float|Truncate (/ (.y (Variables|Default|GetBoxSize)) (Variables|Default|GetDataOffsetDistance))) 1))))))
  (Utilities|Array|Clear (Variables|Default|GetPoints))
  (Spline|ClearSplinePoints (Variables|Default|GetSplinePlotHelper) true)
  (CallFunction|CreateSplinePointsonPlotHelper)
  (CallFunction|CreateSplineMeshGraph)
  (Utilities|FlowControl|Sequence
    (:then_0
      (CallFunction|CreateDynamicGraphMaterials))
    (:then_1
      (CallFunction|SetupGraphSizing))
    (:then_2
      (CallFunction|SetGraphMeshestoNewMaterials))
    (:then_3
      (Class|SplineGraphLocationBucket|CreateSplineGraphLocationBuckets _splinegraphlocationbucket_2 _returnvalue (Variables|/Script/Engine.BoxComponent|GetBoxExtent (Variables|Default|GetBox)) 8 (Variables|Default|GetXGraph))
      (for _index (range 0 50)
        (Class|SplineGraphLocationBucket|AddEntitytoBucket _splinegraphlocationbucket_2 (+ _returnvalue (Math|Vector|MakeVector (* _index 5) 0.0 0.0)))
        (bind _returnvalue_7 (Class|SplineGraphLocationBucket|GetTotalEntitiesinSegmentBucket _splinegraphlocationbucket_2)))
      (Utilities|FlowControl|Sequence
        (:then_0
          (bind _returnvalue_8 (Class|SplineGraphLocationBucket|GetTotalEntitiesinSegmentBucket _splinegraphlocationbucket))
          (Development|PrintString (Utilities|String|Append "Bucket 0 -Number of entities: " (Utilities|String|ToString(Integer) _returnvalue_8))))
        (:then_1
          (bind _returnvalue_9 (Class|SplineGraphLocationBucket|GetTotalEntitiesinSegmentBucket _splinegraphlocationbucket 1))
          (Development|PrintString (Utilities|String|Append "Bucket 1 -Number of entities: " (Utilities|String|ToString(Integer) _returnvalue_9))))
        (:then_2
          (bind _returnvalue_10 (Class|SplineGraphLocationBucket|GetTotalEntitiesinSegmentBucket _splinegraphlocationbucket 2))
          (Development|PrintString (Utilities|String|Append "Bucket 2 -Number of entities: " (Utilities|String|ToString(Integer) _returnvalue_10))))
        (:then_3
          (bind _returnvalue_11 (Class|SplineGraphLocationBucket|GetTotalEntitiesinSegmentBucket _splinegraphlocationbucket 3))
          (Development|PrintString (Utilities|String|Append "Bucket 3 -Number of entities: " (Utilities|String|ToString(Integer) _returnvalue_11))))
        (:then_4
          (bind _returnvalue_12 (Class|SplineGraphLocationBucket|GetTotalEntitiesinSegmentBucket _splinegraphlocationbucket 4))
          (Development|PrintString (Utilities|String|Append "Bucket 4 -Number of entities: " (Utilities|String|ToString(Integer) _returnvalue_12))))
        (:then_5
          (bind _returnvalue_13 (Class|SplineGraphLocationBucket|GetTotalEntitiesinSegmentBucket _splinegraphlocationbucket 5))
          (Development|PrintString (Utilities|String|Append "Bucket 5 -Number of entities: " (Utilities|String|ToString(Integer) _returnvalue_13))))
        (:then_6
          (bind _returnvalue_14 (Class|SplineGraphLocationBucket|GetTotalEntitiesinSegmentBucket _splinegraphlocationbucket 6))
          (Development|PrintString (Utilities|String|Append "Bucket 6 -Number of entities: " (Utilities|String|ToString(Integer) _returnvalue_14))))
        (:then_7
          (bind _returnvalue_15 (Class|SplineGraphLocationBucket|GetTotalEntitiesinSegmentBucket _splinegraphlocationbucket 7))
          (Development|PrintString (Utilities|String|Append "Bucket 7 -Number of entities: " (Utilities|String|ToString(Integer) _returnvalue_15))))
        (:then_8
          (CallFunction|UpdateSplinePoint _returnvalue_3 (Math|Vector|MakeVector (.x (.position _returnvalue_4)) (.y (.position _returnvalue_4)) (* (+ (.Z (Math|Vector|BreakVector _returnvalue)) 2e+01) _returnvalue_7)) (.arrivetangent _returnvalue_4))
          (for _index_2 (range 0 _returnvalue_3)
            (CallFunction|UpdateSplineMeshComponent _index_2)))))))

(fn SetGraphMatColors
  (params (XScale :type Float%20%28single-precision%29) (YScale :type Float%20%28single-precision%29) (Material :type Material%20Instance%20Dynamic%20Object%20Reference) (GraphBackgroundColor :type Linear%20Color%20Structure) (GraphBackgroundLineColor :type Linear%20Color%20Structure) (Masked? :type Float%20%28single-precision%29))
  (Utilities|FlowControl|Sequence
    (:then_0
      (Rendering|Material|SetScalarParameterValue Material "XScale" YScale :!class /Script/Engine.MaterialInstanceDynamic))
    (:then_1
      (Rendering|Material|SetScalarParameterValue Material "YScale" XScale :!class /Script/Engine.MaterialInstanceDynamic))
    (:then_2
      (Rendering|Material|SetVectorParameterValue Material "GraphBackgroundColor" GraphBackgroundColor :!class /Script/Engine.MaterialInstanceDynamic))
    (:then_3
      (Rendering|Material|SetVectorParameterValue Material "GraphBackgroundLineColor" GraphBackgroundLineColor :!class /Script/Engine.MaterialInstanceDynamic))
    (:then_4
      (Rendering|Material|SetScalarParameterValue Material "Masked?" Masked? :!class /Script/Engine.MaterialInstanceDynamic)
      (return))))

(fn CreateSplinePointsonPlotHelper
  (bind _boxsize (Variables|Default|GetBoxSize))
  (bind _returnvalue (Math|Random|RandomFloatinRange 0.0 (.z _boxsize)))
  (for _index (range 0 (- (Variables|Default|GetNumberOfDataPoints) 1))
    (Utilities|GraphType-XTop
      (:X-Axis
        (LocalVariables|SetCurrentPointPos (Math|Vector|MakeVector (* (Variables|Default|GetDataOffsetDistance) _index) 0.0 _returnvalue)))
      (:Y-Axis
        (LocalVariables|SetCurrentPointPos (Math|Vector|MakeVector 0.0 (* (Variables|Default|GetDataOffsetDistance) _index) _returnvalue))))
    (Utilities|Array|Add (Variables|Default|GetPoints) (Utilities|Struct|MakeSplinePoint (Math|Conversions|ToFloat(Integer) _index) (- (LocalVariables|GetCurrentPointPos) (Variables|Default|GetStartPos)) "0.000000,0.000000,0.000000" "0.000000,0.000000,0.000000" "0.000000,0.000000,0.000000" "1.000000,1.000000,1.000000" "Linear")))
  (Class|SplineComponent|AddPoints (Variables|Default|GetSplinePlotHelper) (Variables|Default|GetPoints) true))

(fn CreateSplineMeshGraph
  (bind _meshscale (Variables|Default|GetMeshScale))
  (bind _points (Variables|Default|GetPoints))
  (for (_array_element _array_index) _points
    (LocalVariables|SetLastPoint? (== _array_index (- (Utilities|Array|Length _points) 1)))
    (bind _returnvalue (AddComponent|AddSplineMeshComponent false))
    (bind _output_get (LocalVariables|SetCurrentSplineMesh _returnvalue))
    (SplineMesh|SetForwardAxis _output_get (Variables|Default|GetMeshForward%20Axis) true)
    (Utilities|FlowControl|Sequence
      (:then_0
        (Components|StaticMesh|SetStaticMesh (LocalVariables|GetCurrentSplineMesh) (Variables|Default|GetMeshToUseForGraph))
        (SplineMesh|SetStartTangent (LocalVariables|GetCurrentSplineMesh) (.ArriveTangent (Utilities|Struct|BreakSplinePoint _array_element)) true :!class /Script/Engine.SplineMeshComponent)
        (SplineMesh|SetEndTangent (LocalVariables|GetCurrentSplineMesh) (.LeaveTangent (Utilities|Struct|BreakSplinePoint _array_element)) true :!class /Script/Engine.SplineMeshComponent))
      (:then_1
        (Utilities|GraphType-YTop
          (:Y-Axis
            (SplineMesh|SetStartPosition (LocalVariables|GetCurrentSplineMesh) (.Position (Utilities|Struct|BreakSplinePoint _array_element)) true))
          (:X-Axis
            (SplineMesh|SetStartPosition (.CurrentSplineMesh (Utilities|X-AxisSplineMeshOffset (.Position (Utilities|Struct|BreakSplinePoint _array_element)) (LocalVariables|GetCurrentSplineMesh))) (.OffsetPos (Utilities|X-AxisSplineMeshOffset (.Position (Utilities|Struct|BreakSplinePoint _array_element)) (LocalVariables|GetCurrentSplineMesh))) true))))
      (:then_2
        (SplineMesh|SetStartScale (LocalVariables|GetCurrentSplineMesh) _meshscale true :!class /Script/Engine.SplineMeshComponent))
      (:then_3
        (SplineMesh|SetEndScale (LocalVariables|GetCurrentSplineMesh) _meshscale true :!class /Script/Engine.SplineMeshComponent))
      (:then_4
        (if (LocalVariables|GetLastPoint?)
          (SplineMesh|SetEndPosition (LocalVariables|GetCurrentSplineMesh) (.Position (Utilities|Struct|BreakSplinePoint _array_element)) true)
          (else
            (Utilities|GraphType-YTop
              (:Y-Axis
                (SplineMesh|SetEndPosition (LocalVariables|GetCurrentSplineMesh) (.position (Utilities|Array|Get(acopy) _points (+ _array_index 1))) true))
              (:X-Axis
                (SplineMesh|SetEndPosition (.CurrentSplineMesh (Utilities|X-AxisSplineMeshOffset (.position (Utilities|Array|Get(acopy) _points (+ _array_index 1))) (LocalVariables|GetCurrentSplineMesh))) (.OffsetPos (Utilities|X-AxisSplineMeshOffset (.position (Utilities|Array|Get(acopy) _points (+ _array_index 1))) (LocalVariables|GetCurrentSplineMesh))) true))))))
      (:then_5
        (Utilities|Array|Add (Variables|Default|GetGraphSplineMesh) (LocalVariables|GetCurrentSplineMesh))))))

(fn CreateDynamicGraphMaterials
  (bind _graphbackground (Variables|Default|GetGraphBackGround))
  (bind _xaxis (Variables|Default|GetXAxis))
  (bind _yaxis (Variables|Default|GetYAxis))
  (Utilities|FlowControl|Sequence
    (:then_0
      (bind _returnvalue (Rendering|Material|CreateDynamicMaterialInstance _graphbackground 0 (Rendering|Material|GetMaterial _graphbackground 0) "Graph" :!class /Script/Engine.PrimitiveComponent))
      (Variables|Default|SetGraphBackGroundDynamicMat _returnvalue))
    (:then_1
      (bind _returnvalue_2 (Rendering|Material|CreateDynamicMaterialInstance _xaxis 0 (Rendering|Material|GetMaterial _xaxis 0) "XAxis" :!class /Script/Engine.PrimitiveComponent))
      (Variables|Default|SetGraphSideXAxisDynamicMatInst _returnvalue_2))
    (:then_2
      (bind _returnvalue_3 (Rendering|Material|CreateDynamicMaterialInstance _yaxis 0 (Rendering|Material|GetMaterial _yaxis 0) "YAxis" :!class /Script/Engine.PrimitiveComponent))
      (Variables|Default|SetGraphSideYAxisDynamicMatInst _returnvalue_3))))

(fn SetupGraphSizing
  (bind _numberofdatapoints (Variables|Default|GetNumberOfDataPoints))
  (bind _gridlinecolor (Variables|Default|GetGridLineColor))
  (bind _axis_background_color_and_opacity (Variables|Default|GetAxis%20Background%20Color%20and%20Opacity))
  (bind _returnvalue (- _numberofdatapoints 1))
  (bind _returnvalue_2 (/ _returnvalue 2))
  (bind _returnvalue_3 (Math|Conversions|ToFloat(Integer) _returnvalue_2))
  (Utilities|FlowControl|Sequence
    (:then_0
      (CallFunction|SetGraphMatColors _returnvalue_3 _returnvalue_3 (Variables|Default|GetGraphBackGroundDynamicMat) (Variables|Default|GetGraph%20Background%20Color%20and%20Opacity) _gridlinecolor 0.0))
    (:then_1
      (CallFunction|SetGraphMatColors 0.5 _returnvalue_3 (Variables|Default|GetGraphSideXAxisDynamicMatInst) _axis_background_color_and_opacity _gridlinecolor 1.0))
    (:then_2
      (CallFunction|SetGraphMatColors 0.5 _returnvalue_3 (Variables|Default|GetGraphSideYAxisDynamicMatInst) _axis_background_color_and_opacity _gridlinecolor 1.0))))

(fn SetGraphMeshestoNewMaterials
  (Utilities|FlowControl|Sequence
    (:then_0
      (Rendering|Material|SetMaterial (Variables|Default|GetGraphBackGround) 0 (Variables|Default|GetGraphBackGroundDynamicMat)))
    (:then_1
      (Rendering|Material|SetMaterial (Variables|Default|GetXAxis) 0 (Variables|Default|GetGraphSideXAxisDynamicMatInst)))
    (:then_2
      (Rendering|Material|SetMaterial (Variables|Default|GetYAxis) 0 (Variables|Default|GetGraphSideYAxisDynamicMatInst)))))

(fn UpdateSplinePoint
  (params (PointIndex :type Integer) (InLocation :type Vector%20%28by%20ref%29) (InTangent :type Vector%20%28by%20ref%29))
  (bind _points (Variables|Default|GetPoints))
  (bind _output (Utilities|Array|Get(acopy) _points PointIndex))
  (bind (_inputkey _position _arrivetangent _leavetangent _rotation _scale _type) (Utilities|Struct|BreakSplinePoint _output))
  (Spline|SetLocationatSplinePoint (Variables|Default|GetSplinePlotHelper) PointIndex InLocation "Local" true)
  (|SetBy-RefVar _output (Utilities|Struct|MakeSplinePoint _inputkey InLocation "0.000000,0.000000,0.000000" "0.000000,0.000000,0.000000" _rotation _scale _type))
  (return))

(fn UpdateSplineMeshComponent
  (params (Index :type Integer))
  (bind _returnvalue (+ Index 1))
  (bind _graphsplinemesh (Variables|Default|GetGraphSplineMesh))
  (bind _points (Variables|Default|GetPoints))
  (bind _points_2 (Variables|Default|GetPoints))
  (bind _output (Utilities|Array|Get(acopy) _graphsplinemesh Index))
  (bind _output_2 (Utilities|Array|Get(acopy) _points_2 Index))
  (bind _output_3 (Utilities|Array|Get(acopy) _points Index))
  (bind _output_4 (Utilities|Array|Get(acopy) _points _returnvalue))
  (bind (_currentsplinemesh _offsetpos) (Utilities|X-AxisSplineMeshOffset (.position _output_2) _output))
  (bind (_currentsplinemesh_2 _offsetpos_2) (Utilities|X-AxisSplineMeshOffset (.position _output_4) _output))
  (if (== (- (Utilities|Array|Length _points) 1) Index)
    (Utilities|GraphType-YTop
      (:Y-Axis
        (SplineMesh|SetStartandEnd _output (.position _output_2) "0, 0, 0" (.position _output_2) "0, 0, 0" true :!class /Script/Engine.SplineMeshComponent))
      (:X-Axis
        (SplineMesh|SetStartandEnd _currentsplinemesh _offsetpos "0, 0, 0" _offsetpos "0, 0, 0" true :!class /Script/Engine.SplineMeshComponent)))
    (else
      (Utilities|GraphType-YTop
        (:Y-Axis
          (SplineMesh|SetStartandEnd _output (.position _output_3) "0, 0, 0" (.position _output_4) "0, 0, 0" true :!class /Script/Engine.SplineMeshComponent))
        (:X-Axis
          (SplineMesh|SetStartandEnd _currentsplinemesh_2 (.OffsetPos (Utilities|X-AxisSplineMeshOffset (.position _output_3) _output)) "0, 0, 0" _offsetpos_2 "0, 0, 0" true :!class /Script/Engine.SplineMeshComponent))))))