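; Test Blueprint for rendering a Voronoi diagram onto a plane through a dynamic pixel texture.
; As wired, BeginPlay does nothing and the construction script only clears DataPoints.
; Two disconnected chains, one per graph, scatter random points, build a relaxed diagram with DynamicPixelRenderingTexture and apply it via an M_VoronoiMap dynamic material.
; They differ in texture size, point count and clear/update order, and neither runs.
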(event EventBeginPlay)

(fn ConstructionScript
  (Utilities|Array|Clear (Variables|Default|GetData%20Points)))