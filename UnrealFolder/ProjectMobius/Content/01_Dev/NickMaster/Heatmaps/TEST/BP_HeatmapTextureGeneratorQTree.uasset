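; Test variant of a heatmap texture generator that exercises quadtree-backed heatmap updates, though none of its logic currently runs.
; BeginPlay and the construction script are empty, leaving all test chains disconnected.
; The main unused chain builds a BP_QuadTreeTest tree from HeatmapMesh bounds and inserts diagonally stepped sample locations.
; It then alternates two point sets through UpdateHeatmapWithMultipleAgents with delays; smaller leftover chains call UpdateHeatmap on single points.
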(event EventBeginPlay)

(fn ConstructionScript)