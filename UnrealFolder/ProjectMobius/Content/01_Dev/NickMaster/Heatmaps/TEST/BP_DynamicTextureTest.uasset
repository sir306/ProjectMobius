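; Test actor for drawing heatmaps into a runtime DynamicPixelRenderingTexture shown on a Plane; all its logic is disconnected, so BeginPlay and construction do nothing.
; The main unwired construction chain binds the texture to an M_HeatmapRT_V2 dynamic material and draws a circle at LocationWorld scaled to pixels.
; It then converts the texture to RGB and updates the render.
; Other loose fragments try line drawing, M_VoronoiMap and bounds printing.
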(event EventBeginPlay)

(fn ConstructionScript)