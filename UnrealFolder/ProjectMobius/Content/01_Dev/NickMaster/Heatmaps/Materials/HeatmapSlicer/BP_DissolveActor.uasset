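; BP_DissolveActor is a box volume actor that feeds its cube's placement to materials for a box dissolve effect, filed under the heatmap slicer materials.
; It writes the Cube component's world location and full bounds size into the MPC_BoxDissolveParamCollection material parameter collection.
; The write runs in both the construction script and BeginPlay, with no per-frame update.
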(event EventBeginPlay
  (bind _cube (Variables|Default|GetCube))
  (Rendering|Material|SetVectorParameterValue "/Game/01_Dev/NickMaster/Heatmaps/Materials/HeatmapSlicer/MPC_BoxDissolveParamCollection.MPC_BoxDissolveParamCollection" "Location" (Math|Conversions|ToLinearColor(Vector) (Transformation|GetWorldLocation _cube)) :!class /Script/Engine.KismetMaterialLibrary)
  (Rendering|Material|SetVectorParameterValue "/Game/01_Dev/NickMaster/Heatmaps/Materials/HeatmapSlicer/MPC_BoxDissolveParamCollection.MPC_BoxDissolveParamCollection" "Bounds" (Math|Conversions|ToLinearColor(Vector) (* (.BoxExtent (Collision|GetComponentBounds _cube)) 2)) :!class /Script/Engine.KismetMaterialLibrary))

(event Collision|EventActorBeginOverlap
  (params (OtherActor :type Actor%20Object%20Reference)))

(event EventTick
  (params (DeltaSeconds :type Float%20%28single-precision%29)))

(fn ConstructionScript
  (bind _cube (Variables|Default|GetCube))
  (Rendering|Material|SetVectorParameterValue "/Game/01_Dev/NickMaster/Heatmaps/Materials/HeatmapSlicer/MPC_BoxDissolveParamCollection.MPC_BoxDissolveParamCollection" "Location" (Math|Conversions|ToLinearColor(Vector) (Transformation|GetWorldLocation _cube)) :!class /Script/Engine.KismetMaterialLibrary)
  (Rendering|Material|SetVectorParameterValue "/Game/01_Dev/NickMaster/Heatmaps/Materials/HeatmapSlicer/MPC_BoxDissolveParamCollection.MPC_BoxDissolveParamCollection" "Bounds" (Math|Conversions|ToLinearColor(Vector) (* (.BoxExtent (Collision|GetComponentBounds _cube)) 2)) :!class /Script/Engine.KismetMaterialLibrary))